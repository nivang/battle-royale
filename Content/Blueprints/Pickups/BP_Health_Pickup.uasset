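; BP_Health_Pickup is a pickup that heals a character who enters its pickup sphere.
; On authority only, PickupSphereEntered checks that the character's health is below maximum, then passes a negated HealthToGive to ModifyHealth and destroys the pickup.
; Characters at full health leave the pickup in place.
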(event `/Game/Blueprints/Pickups/BP_Pickup.Pickup Sphere Entered`
  (params (Character :type "/Game/FirstPersonBP/Blueprints/BRCharacter Object Reference"))
  (`/Engine/EditorBlueprintResources/ActorMacros.Switch Has Authority`
    (:`Authority`
      (if (< (`/Game/FirstPersonBP/Blueprints/BRCharacter.Health` Character) (`/Game/FirstPersonBP/Blueprints/BRCharacter.MaxHealth` Character))
        (`/Game/FirstPersonBP/Blueprints/BRCharacter.Modify Health` Character (* (`self.HealthToGive`) -1.0))
        (`self.K2_DestroyActor`)))))

(fn `UserConstructionScript`
  (`parent.UserConstructionScript`))